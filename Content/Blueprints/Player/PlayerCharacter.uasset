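; Player character Blueprint that handles pausing and health bar updates.
; Escape or NumPad Six creates a PauseMenu widget, adds it to the viewport, pauses the game and shows the mouse cursor.
; When HealthComponent signals a life change, its life percentage is written to the ProgressionPercent of the HealthBar widget, obtained by casting the widget held by the HealthBar component.
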(event OnLifeChanged(healthComponent)
  (params (newLife :type Integer))
  (bind _ashealth_bar (Utilities|Casting|CastToHealthBar (UserInterface|GetWidget (Variables|Default|GetHealthBar))))
  (bind _returnvalue (Class|LifeComponent|GetLifePercent (Variables|Default|GethealthComponent)))
  (Variables|/Game/Blueprints/HealthBar.HealthBar_C|SetprogressionPercent _ashealth_bar _returnvalue))

(event Input|KeyboardEvents|Escape
  (params (Key :type Key%20Structure :default "None"))
  (:Pressed
    (bind _returnvalue (UserInterface|CreateWidget "/Game/Blueprints/UIs/PauseMenu.PauseMenu_C"))
    (UserInterface|Viewport|AddtoViewport _returnvalue 0)
    (Game|SetGamePaused true)
    (Variables|/Script/Engine.PlayerController|SetbShowMouseCursor (Game|GetPlayerController 0) true)))

(event Input|KeyboardEvents|NumPadSix
  (params (Key :type Key%20Structure :default "None"))
  (:Pressed
    (bind _returnvalue (UserInterface|CreateWidget "/Game/Blueprints/UIs/PauseMenu.PauseMenu_C"))
    (UserInterface|Viewport|AddtoViewport _returnvalue 0)
    (Game|SetGamePaused true)
    (Variables|/Script/Engine.PlayerController|SetbShowMouseCursor (Game|GetPlayerController 0) true)))

(fn ConstructionScript)