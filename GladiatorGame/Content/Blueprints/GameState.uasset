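; GameState Blueprint that handles the end of a match by showing the victory or game over screen.
; On BeginPlay it binds its GameTerminate event to OnGameTerminate.
; When fired, the event waits briefly, adds the VictoryMenu or GameOverMenu widget to the viewport based on the Victory flag, then pauses the game and shows the mouse cursor.
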(event Custom|GameTerminate
  (params (victory :type Boolean))
  (Utilities|FlowControl|Delay 2.0)
  (if victory
    (bind _returnvalue (UserInterface|CreateWidget "/Game/Blueprints/UIs/VictoryMenu.VictoryMenu_C"))
    (UserInterface|Viewport|AddtoViewport _returnvalue 0)
    (else
      (bind _returnvalue_2 (UserInterface|CreateWidget "/Game/Blueprints/UIs/GameOverMenu.GameOverMenu_C"))
      (UserInterface|Viewport|AddtoViewport _returnvalue_2 0)))
  (Game|SetGamePaused true)
  (Variables|/Script/Engine.PlayerController|SetbShowMouseCursor (Game|GetPlayerController 0) true))

(event EventBeginPlay
  (EventDispatchers|BindEventtoOnGameTerminate (EventDispatchers|CreateEvent :!event Custom|GameTerminate)))

(fn ConstructionScript)